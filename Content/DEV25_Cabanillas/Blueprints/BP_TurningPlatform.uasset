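; BP_TurningPlatform is an actor that repeatedly flips 180 degrees around a configurable axis, pausing for a configurable delay between turns.
; Each turn stores the starting rotation, then a timeline lerps the current rotation toward that start combined with the half-turn, looping from BeginPlay.
; A Box component respawns any BP_CustomThirdPersonCharacter that begins overlapping it.
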(event OnComponentBeginOverlap(Box)
  (params (OverlappedComponent :type Primitive%20Component%20Object%20Reference) (OtherActor :type Actor%20Object%20Reference) (OtherComp :type Primitive%20Component%20Object%20Reference) (OtherBodyIndex :type Integer) (bFromSweep :type Boolean) (SweepResult :type Hit%20Result%20Structure%20%28by%20ref%29))
  (bind _asbp_custom_third_person_character (Utilities|Casting|CastToBP_CustomThirdPersonCharacter OtherActor))
  (Default|Respawn _asbp_custom_third_person_character))

(event Custom|Rotate
  (bind _returnvalue (Transformation|GetActorRotation))
  (Variables|Default|SetStartChangeRotation _returnvalue)
  (bind _rotate (Timeline|RotateTimeline PlayFromStart)
    (:Update
      (Transformation|SetActorRotation (Math|Rotator|Lerp(Rotator) _returnvalue (Math|Rotator|CombineRotators (Variables|Default|GetStartChangeRotation) (Math|Vector|RotatorfromAxisandAngle (Variables|Default|GetAxis) 1.8e+02)) _rotate)))
    (:Finished
      (Utilities|FlowControl|Delay (Variables|Default|GetChangeDelay))
      (CallFunction|Rotate))))

(event EventBeginPlay
  (CallFunction|Rotate))

(fn ConstructionScript)