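; BP_GoalPlatformButton is a one-shot trigger that moves a linked goal platform into position while showing it through a cinematic camera.
; On the first Box overlap, it switches the player's view to the CinematicCamera, calls SetToPosition on the RelatedGoalPlatform and sets HasBeenActivated.
; After a three-second delay, it returns the view to the owner of the player character's camera.
; The overlap does not filter which actor triggers it.
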(event OnComponentBeginOverlap(Box)
  (params (OverlappedComponent :type Primitive%20Component%20Object%20Reference) (OtherActor :type Actor%20Object%20Reference) (OtherComp :type Primitive%20Component%20Object%20Reference) (OtherBodyIndex :type Integer) (bFromSweep :type Boolean) (SweepResult :type Hit%20Result%20Structure%20%28by%20ref%29))
  (bind _returnvalue (Game|GetPlayerController 0))
  (if (not (Variables|Default|GetHasBeenActivated))
    (bind _asbp_goal_platform (Utilities|Casting|CastToBP_GoalPlatform (Variables|Default|GetRelatedGoalPlatform)))
    (bind _ascamera_actor (Utilities|Casting|CastToCameraActor (Variables|Default|GetCinematicCamera)))
    (Game|Player|SetViewTargetwithBlend _returnvalue _ascamera_actor 0.0 "VTBlend_Linear" 0.0 false)
    (Default|SettoPosition _asbp_goal_platform)
    (Variables|Default|SetHasBeenActivated true)
    (Utilities|FlowControl|Delay 3.0)
    (bind _asbp_custom_third_person_character (Utilities|Casting|CastToBP_CustomThirdPersonCharacter (Game|Player|GetPlayerPawn 0)))
    (bind _camera (Default|GetCamera _asbp_custom_third_person_character))
    (Game|Player|SetViewTargetwithBlend _returnvalue (Components|GetOwner _camera) 0.0 "VTBlend_Linear" 0.0 false)))

(event EventBeginPlay)

(event Collision|EventActorBeginOverlap
  (params (OtherActor :type Actor%20Object%20Reference)))

(event EventTick
  (params (DeltaSeconds :type Float%20%28single-precision%29)))

(fn ConstructionScript)