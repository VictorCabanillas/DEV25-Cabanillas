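; BP_GoalPlatform is a platform actor that stays hidden far below its placed spot until it is told to rise into position.
; BeginPlay saves the placed location, then drops the actor 1000 units down.
; SetToPosition triggers MovePlatformEvent, whose MovePlatform timeline lerps from the current location toward the saved start, so the motion eases in cumulatively rather than following the raw alpha.
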(event Custom|MovePlatformEvent
  (bind _alpha (Timeline|MovePlatform Play)
    (:Update
      (Transformation|SetActorLocation (Math|Vector|Lerp(Vector) (Transformation|GetActorLocation) (Variables|Default|GetStartPos) _alpha) false false))))

(event EventBeginPlay
  (bind _returnvalue (Transformation|GetActorLocation))
  (Variables|Default|SetStartPos _returnvalue)
  (Transformation|SetActorLocation (+ _returnvalue "0.000000,0.000000,-1000.000000") false false))

(fn ConstructionScript)

(fn SettoPosition
  (CallFunction|MovePlatformEvent))